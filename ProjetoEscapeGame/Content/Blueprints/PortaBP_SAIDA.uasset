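; PortaBP_SAIDA is a door, named as the exit, that the player opens and closes with Interact while holding the item matching IdPeDeCabra (crowbar).
; A Box overlap enables input on the actor only while something is inside it.
; Interact checks the FirstPersonCharacter's EquippedItem, then plays or reverses a timeline based on its current value.
; The timeline output sets the Porta component's relative yaw.
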(event OnComponentBeginOverlap(Box)
  (params (OverlappedComponent :type Primitive%20Component%20Object%20Reference) (OtherActor :type Actor%20Object%20Reference) (OtherComp :type Primitive%20Component%20Object%20Reference) (OtherBodyIndex :type Integer) (bFromSweep :type Boolean) (SweepResult :type Hit%20Result%20Structure%20%28by%20ref%29))
  (Input|EnableInput (Game|GetPlayerController 0)))

(event OnComponentEndOverlap(Box)
  (params (OverlappedComponent :type Primitive%20Component%20Object%20Reference) (OtherActor :type Actor%20Object%20Reference) (OtherComp :type Primitive%20Component%20Object%20Reference) (OtherBodyIndex :type Integer))
  (Input|DisableInput (Game|GetPlayerController 0)))

(event Input|ActionEvents|InputActionInteract
  (params (Key :type Key%20Structure))
  (:Pressed
    (bind _asfirst_person_character (Utilities|Casting|CastToFirstPersonCharacter (Game|GetPlayerCharacter 0)))
    (if (== (.Id (Utilities|Struct|BreakItemDataStruct (Variables|/Game/FirstPersonBP/Blueprints/FirstPersonCharacter.FirstPersonCharacter_C|GetEquippedItem _asfirst_person_character))) (Variables|Default|GetId_Pe_de_Cabra))
      (if (< (stale _abrir_fechar_porta) 1.0)
        (bind _abrir_fechar_porta (Timeline|Linha%20do%20Tempo_0 Play)
          (:Update
            (Transformation|SetRelativeRotation (Variables|Default|GetPorta) (Math|Rotator|MakeRotator 0.0 0.0 _abrir_fechar_porta) false false)))
        (else
          (Timeline|Linha%20do%20Tempo_0 Reverse))))))

(fn ConstructionScript
  (|CallParentFunction))