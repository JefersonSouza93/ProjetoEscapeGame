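; An interactable object that swaps the player's equipped bucket (Balde) item for another one, BaldeQueSalva.
; On Interact, it checks the FirstPersonCharacter's equipped item ID, replaces the first matching inventory entry and equips the new item.
; It then sends a success message and an equip refresh to the HUD widget, or only a missing-item message when the bucket is not equipped.
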(event EventInteract
  (bind _balde_que_salva (Variables|Default|Getbalde_que_salva))
  (bind _asfirst_person_character (Utilities|Casting|CastToFirstPersonCharacter (Game|GetPlayerCharacter 0)))
  (if (== (.Id (Utilities|Struct|BreakItemDataStruct (Variables|/Game/FirstPersonBP/Blueprints/FirstPersonCharacter.FirstPersonCharacter_C|GetEquippedItem _asfirst_person_character))) (Variables|Default|GetId_Balde))
    (bind (_array_element _array_index) (Utilities|Array|ForEachLoopwithBreak (Variables|/Game/FirstPersonBP/Blueprints/FirstPersonCharacter.FirstPersonCharacter_C|GetInventory _asfirst_person_character) :!label _label)
      (:LoopBody
        (if (== (.Id (Utilities|Struct|BreakItemDataStruct (Utilities|Struct|BreakInventoryStruct _array_element))) (Variables|Default|GetId_Balde))
          (Utilities|Array|RemoveIndex (Variables|/Game/FirstPersonBP/Blueprints/FirstPersonCharacter.FirstPersonCharacter_C|GetInventory _asfirst_person_character) _array_index)
          (Utilities|Array|Add (Variables|/Game/FirstPersonBP/Blueprints/FirstPersonCharacter.FirstPersonCharacter_C|GetInventory _asfirst_person_character) _balde_que_salva)
          (Variables|/Game/FirstPersonBP/Blueprints/FirstPersonCharacter.FirstPersonCharacter_C|SetEquippedItem _asfirst_person_character (Utilities|Struct|BreakInventoryStruct _balde_que_salva))
          (goto _label Break)))
      (:Completed
        (bind _foundwidgets (Widget|GetAllWidgetsOfClass "/Game/FirstPersonBP/Blueprints/HUDWidget.HUDWidget_C" true))
        (Default|HUDMessage _foundwidgets (Variables|Default|GetHas_Item_Message))
        (Default|OnEquip _foundwidgets)))
    (else
      (bind _foundwidgets_2 (Widget|GetAllWidgetsOfClass "/Game/FirstPersonBP/Blueprints/HUDWidget.HUDWidget_C" true))
      (Default|HUDMessage _foundwidgets_2 (Variables|Default|GetNo_Item_HUD_text)))))

(fn ConstructionScript)